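; BP_Invincible is the invincibility effect for the player, showing a spinning Body for a limited time.
; Activate shows the Body, plays the skill sound at its location and starts the active state.
; Tick rotates the Body every frame and, once ActiveTime elapses, hides it and clears Invincible on the cached BP_ThirdPersonCharacter.
; The flag is only cleared here, never set.
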(event `self.ReceiveBeginPlay`
  (bind _asbp_third_person_character (cast `/Game/ThirdPerson/Blueprints/BP_ThirdPersonCharacter` (`GameplayStatics.GetPlayerPawn` 0)))
  (set `self.Third Person Character` _asbp_third_person_character))

(event `self.ReceiveTick`
  (params (DeltaSeconds :type "Float (single-precision)"))
  (`SceneComponent.K2_AddWorldRotation` (`self.Body`) (struct :`Pitch` 10.0 :`Yaw` 10.0 :`Roll` 10.0) false false)
  (if (`self.Activated`)
    (bind _output_get (set `self.Timer` (+ (`self.Timer`) (`GameplayStatics.GetWorldDeltaSeconds`))))
    (if (>= _output_get (`self.ActiveTime`))
      (set `self.Activated` false)
      (set `self.Timer` 0.0)
      (`SceneComponent.SetVisibility` (`self.Body`) false false)
      (set `/Game/ThirdPerson/Blueprints/BP_ThirdPersonCharacter.Invincible` false (`self.Third Person Character`)))))

(fn `Activate`
  (`SceneComponent.SetVisibility` (`self.Body`) true false)
  (set `self.Activated` true)
  (`GameplayStatics.PlaySoundAtLocation` "/Game/Resources/Sound/InvicibleSkill.InvicibleSkill" (`SceneComponent.K2_GetComponentLocation` (`self.Body`)) (struct) 1.0 1.0 0.0 null null null null))

(fn `UserConstructionScript`)