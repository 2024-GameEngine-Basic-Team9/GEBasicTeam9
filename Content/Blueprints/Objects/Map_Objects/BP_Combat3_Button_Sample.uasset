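; BP_Combat3_Button_Sample is a map button that toggles its look whenever the third-person player character overlaps it.
; On BeginPlay it gives the Cylinder mesh a dynamic instance of the sample button material.
; Each qualifying overlap flips the Glowing flag and switches the material's "B" scalar parameter between two values.
; The toggle is purely visual, with no other gameplay logic in the Blueprint.
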(event `self.ReceiveBeginPlay`
  (bind _returnvalue (`PrimitiveComponent.CreateDynamicMaterialInstance` (`self.Cylinder`) 0 "/Game/Blueprints/Objects/Map_Objects/Button_Sample_material.Button_Sample_material" "None"))
  (bind _output_get (set `self.DynamicColor` _returnvalue))
  (`PrimitiveComponent.SetMaterial` (`self.Cylinder`) 0 _output_get)
  (`MaterialInstanceDynamic.SetScalarParameterValue` _output_get "B" 0.1))

(event `self.ReceiveActorBeginOverlap`
  (params (OtherActor :type "Actor Object Reference"))
  (bind _dynamiccolor (`self.DynamicColor`))
  (cast `/Game/ThirdPerson/Blueprints/BP_ThirdPersonCharacter` OtherActor)
  (bind _output_get (set `self.Glowing` (not (`self.Glowing`))))
  (if _output_get
    (`MaterialInstanceDynamic.SetScalarParameterValue` _dynamiccolor "B" 0.0)
    (else
      (`MaterialInstanceDynamic.SetScalarParameterValue` _dynamiccolor "B" 0.1))))

(fn `UserConstructionScript`)