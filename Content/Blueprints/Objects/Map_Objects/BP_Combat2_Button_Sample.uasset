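; Floor-style button sample actor that toggles a dynamic material parameter and starts a timed countdown when BP_ThirdPersonCharacter overlaps it.
; Activation creates a BP_Timer_Sample widget and an audio component, with OnProgress blocking further reactions while it runs.
; A looping timer scales volume from the widget's limit over remaining time, stopping audio and removing the progress bar near the clamp ceiling.
; SetVolume is an unfinished stub.
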(event `self.ReceiveBeginPlay`
  (bind _returnvalue (`PrimitiveComponent.CreateDynamicMaterialInstance` (`self.Cube`) 0 "/Game/Blueprints/Objects/Map_Objects/Button_Sample_material.Button_Sample_material" "None"))
  (bind _output_get (set `self.DynamicColor` _returnvalue))
  (`PrimitiveComponent.SetMaterial` (`self.Cube`) 0 _output_get)
  (`MaterialInstanceDynamic.SetScalarParameterValue` _output_get "B" 0.1))

(event `self.ReceiveActorBeginOverlap`
  (params (OtherActor :type "Actor Object Reference"))
  (bind _dynamiccolor (`self.DynamicColor`))
  (cast `/Game/ThirdPerson/Blueprints/BP_ThirdPersonCharacter` OtherActor)
  (bind _output_get (set `self.Glowing` (not (`self.Glowing`))))
  (if (`self.OnProgress`)
    _
    (elif _output_get
      (`MaterialInstanceDynamic.SetScalarParameterValue` _dynamiccolor "B" 0.0)
      (bind _returnvalue (`|CreateWidget` "/Game/Blueprints/Objects/Map_Objects/BP_Timer_Sample.BP_Timer_Sample_C" null 7.0 7.0))
      (`UserWidget.AddToViewport` _returnvalue 0)
      (set `self.OnProgress` true)
      (bind _returnvalue_2 (`AddComponent|NODE_AddAudioComponent-1`))
      (`SceneComponent.K2_SetWorldLocation` _returnvalue_2 (0.0 0.0 0.0) false false)
      (if (>= (`KismetMathLibrary.FClamp` (/ (`/Game/Blueprints/Objects/Map_Objects/BP_Timer_Sample.Limit` _returnvalue) (+ (`/Game/Blueprints/Objects/Map_Objects/BP_Timer_Sample.Remain_Time` _returnvalue) 2.0)) 0.0 5.0) 4.9) :!label _label
        (`AudioComponent.Stop` _returnvalue_2)
        (bind _progressbar_0 (`/Game/Blueprints/Objects/Map_Objects/BP_Timer_Sample.ProgressBar_0` _returnvalue))
        (if (`KismetSystemLibrary.IsValid` _progressbar_0)
          (`Widget.RemoveFromParent` _progressbar_0)
          (set `self.OnProgress` false))
        (else
          (`KismetSystemLibrary.K2_SetTimerDelegate` (delegate `Volume_Manage`) 0.1 true)))
      (else
        (`MaterialInstanceDynamic.SetScalarParameterValue` _dynamiccolor "B" 0.1)))))

(event `Volume_Manage`
  (`AudioComponent.SetVolumeMultiplier` (stale `self.ReceiveActorBeginOverlap` _returnvalue_2) (`KismetMathLibrary.FClamp` (/ (`/Game/Blueprints/Objects/Map_Objects/BP_Timer_Sample.Limit` (stale `self.ReceiveActorBeginOverlap` _returnvalue)) (+ (`/Game/Blueprints/Objects/Map_Objects/BP_Timer_Sample.Remain_Time` (stale `self.ReceiveActorBeginOverlap` _returnvalue)) 2.0)) 0.0 5.0))
  (goto _label))

(fn `Set_Volume`
  (if (> (`self.Current_Volume`) 0.0)
    _))

(fn `UserConstructionScript`)