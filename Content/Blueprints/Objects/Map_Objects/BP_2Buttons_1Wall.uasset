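; Puzzle object with two pressure buttons and an electric wall that opens once both buttons are held by third-person characters at the same time.
; Overlap begin and end toggle each button's state and glow through dynamic material instances.
; When both are on, it latches permanently, and a timeline drives the wall's opacity before disabling its collision.
; Button press-movement logic is disconnected, noted as causing an infinite-loop bug.
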(event `self.ReceiveBeginPlay`
  ;[1 1 1] 버튼 이머시브 조정 밑작업
  (bind _returnvalue (`PrimitiveComponent.CreateDynamicMaterialInstance` (`self.Button`) 0 "/Game/Blueprints/Objects/Map_Objects/Button_Sample_material.Button_Sample_material" "None"))
  (bind _returnvalue_2 (`PrimitiveComponent.CreateDynamicMaterialInstance` (`self.Button1`) 0 "/Game/Blueprints/Objects/Map_Objects/Button_Sample_material.Button_Sample_material" "None"))
  (bind _output_get (set `self.DynamicColor` _returnvalue))
  (bind _output_get_2 (set `self.DynamicColor1` _returnvalue_2))
  (`PrimitiveComponent.SetMaterial` (`self.Button`) 0 _output_get)
  (`PrimitiveComponent.SetMaterial` (`self.Button1`) 0 _output_get_2)
  ;[1 1 1] 벽 오파시티 조정 밑작업
  (bind _returnvalue_3 (`PrimitiveComponent.CreateDynamicMaterialInstance` (`self.Cube`) 0 "/Game/Blueprints/Objects/Map_Objects/EletroWall_Sample.EletroWall_Sample" "None"))
  (bind _output_get_3 (set `self.Wall_Dynamic` _returnvalue_3))
  (`PrimitiveComponent.SetMaterial` (`self.Cube`) 0 _output_get_3))

(event `self.Button.OnComponentBeginOverlap`
  (params (OverlappedComponent :type "PrimitiveComponent Object Reference") (OtherActor :type "Actor Object Reference") (OtherComp :type "PrimitiveComponent Object Reference") (OtherBodyIndex :type Integer) (bFromSweep :type Boolean) (SweepResult :type "HitResult Structure (by ref)"))
  (cast `/Game/ThirdPerson/Blueprints/BP_ThirdPersonCharacter` OtherActor)
  ;[1 1 1] 한 번만 작동, 버튼 작동 여부
  (if (`self.IsNew`)
    (if (not (`self.Button_On`))
      (set `self.Button_On` true)
      ;[1 1 1] 버튼 발광
      (`MaterialInstanceDynamic.SetScalarParameterValue` (`self.DynamicColor`) "B" 0.1)
      ;[1 1 1] 동시 작동 여부 확인
      (if (and (`self.Button_On`) (`self.Button1_On`)) :!label _label
        (set `self.IsNew` false)
        ;[1 1 1] 벽 3초에 걸쳐 오파시티 감소 후 No Collision
        (bind (_direction `_새_트랙_0`) (`Timeline|타임라인`)
          (:`Update`
            (`MaterialInstanceDynamic.SetScalarParameterValue` (`self.Wall_Dynamic`) "Opacity" `_새_트랙_0`))
          (:`Finished`
            (`PrimitiveComponent.SetCollisionEnabled` (`self.Cube`) "NoCollision")))))))

(event `self.Button1.OnComponentBeginOverlap`
  (params (OverlappedComponent :type "PrimitiveComponent Object Reference") (OtherActor :type "Actor Object Reference") (OtherComp :type "PrimitiveComponent Object Reference") (OtherBodyIndex :type Integer) (bFromSweep :type Boolean) (SweepResult :type "HitResult Structure (by ref)"))
  (cast `/Game/ThirdPerson/Blueprints/BP_ThirdPersonCharacter` OtherActor)
  (if (`self.IsNew`)
    (if (not (`self.Button1_On`))
      (set `self.Button1_On` true)
      (`MaterialInstanceDynamic.SetScalarParameterValue` (`self.DynamicColor1`) "B" 0.1)
      (goto _label))))

(event `self.Button.OnComponentEndOverlap`
  (params (OverlappedComponent :type "PrimitiveComponent Object Reference") (OtherActor :type "Actor Object Reference") (OtherComp :type "PrimitiveComponent Object Reference") (OtherBodyIndex :type Integer))
  (cast `/Game/ThirdPerson/Blueprints/BP_ThirdPersonCharacter` OtherActor)
  (if (`self.IsNew`)
    (if (`self.Button_On`)
      (set `self.Button_On` false)
      (`MaterialInstanceDynamic.SetScalarParameterValue` (`self.DynamicColor`) "B" 0.0))))

(event `self.Button1.OnComponentEndOverlap`
  (params (OverlappedComponent :type "PrimitiveComponent Object Reference") (OtherActor :type "Actor Object Reference") (OtherComp :type "PrimitiveComponent Object Reference") (OtherBodyIndex :type Integer))
  (cast `/Game/ThirdPerson/Blueprints/BP_ThirdPersonCharacter` OtherActor)
  (if (`self.IsNew`)
    (if (`self.Button1_On`)
      (set `self.Button1_On` false)
      (`MaterialInstanceDynamic.SetScalarParameterValue` (`self.DynamicColor1`) "B" 0.0))))

(fn `ButtonWork`)

(fn `UserConstructionScript`)