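; Floor-trigger button for a timed combat challenge: the player's overlap starts four successive waves of paired targets, each announced by a bell.
; A 0.1-second timer loop polls each pair's Clear flags to spawn the next wave and scales the timer sound's volume as time runs out.
; Clearing all waves fades the electric wall via a timeline and disables its collision.
; Timeout destroys targets, resets progress and extends the next attempt's limit.
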(event `self.ReceiveBeginPlay`
  (bind _returnvalue (`PrimitiveComponent.CreateDynamicMaterialInstance` (`self.Cylinder`) 0 "/Game/Blueprints/Objects/Map_Objects/Button_Sample_material.Button_Sample_material" "None"))
  (bind _output_get (set `self.DynamicColor` _returnvalue))
  (`PrimitiveComponent.SetMaterial` (`self.Cylinder`) 0 _output_get)
  (`MaterialInstanceDynamic.SetScalarParameterValue` _output_get "B" 0.1)
  ;[1 1 1] 벽 오파시티 조정 밑작업
  (bind _returnvalue_2 (`PrimitiveComponent.CreateDynamicMaterialInstance` (`self.Wall_Cube`) 0 "/Game/Blueprints/Objects/Map_Objects/EletroWall_Sample.EletroWall_Sample" "None"))
  (bind _output_get_2 (set `self.Wall_Dynamic` _returnvalue_2))
  (`PrimitiveComponent.SetMaterial` (`self.Wall_Cube`) 0 _output_get_2))

(event `self.ReceiveActorBeginOverlap`
  (params (OtherActor :type "Actor Object Reference"))
  (bind _limit (`self.Limit`))
  (cast `/Game/ThirdPerson/Blueprints/BP_ThirdPersonCharacter` OtherActor)
  (if (`self.IsCleared`)
    _
    (elif (not (`self.OnProgress`))
      (`MaterialInstanceDynamic.SetScalarParameterValue` (`self.DynamicColor`) "B" 0.0)
      ;[1 1 1] 과녁 2개 생성
      (`|ExecutionSequence`
        (:`then_0`
          (bind _returnvalue (`|SpawnActorFromClass` "/Game/Blueprints/Objects/Target/BP_TargetMoving.BP_TargetMoving_C" (`KismetMathLibrary.MakeTransform` (-1690.0 -2830.0 220.0) (struct :`Yaw` -90.0)) "Undefined" "MultiplyWithRoot" null (-1690.0 -2830.0 220.0) (-1690.0 -4230.0 500.0) true null)))
        (:`then_1`
          (bind _returnvalue_2 (`|SpawnActorFromClass` "/Game/Blueprints/Objects/Target/BP_TargetFracture.BP_TargetFracture_C" (`KismetMathLibrary.MakeTransform` (-1390.0 -3850.0 320.0) (struct :`Yaw` 90.0)) "Undefined" "MultiplyWithRoot" null null))
          (`GameplayStatics.PlaySoundAtLocation` "/Game/Blueprints/Objects/Map_Objects/Bell_Sound.Bell_Sound" (-1660.0 -3445.0 200.0) (struct) 1.0 1.5 0.0 "/Game/Blueprints/Objects/Map_Objects/Bell_Attenuation.Bell_Attenuation" null null null)
          ;[1 1 1] 위젯 및 타이머 소리 재생
          (bind _returnvalue_3 (`|CreateWidget` "/Game/Blueprints/Objects/Map_Objects/BP_Timer_Sample.BP_Timer_Sample_C" null _limit _limit))
          (bind _output_get (set `self.BP_Widget` _returnvalue_3))
          (`UserWidget.AddToViewport` _output_get 0)
          (set `self.OnProgress` true)
          (bind _returnvalue_4 (`AddComponent|NODE_AddAudioComponent-1`))
          (if (or (>= 0.0 (`/Game/Blueprints/Objects/Map_Objects/BP_Timer_Sample.Remain_Time` _output_get)) (stale `Volume_Manage` _output_get)) :!label _label
            (`AudioComponent.Stop` _returnvalue_4)
            (if (`KismetSystemLibrary.IsValid` _returnvalue_3)
              (`Widget.RemoveFromParent` _returnvalue_3)
              (set `self.OnProgress` false)
              (if (`self.IsCleared`)
                ;[1 1 1] (클리어 보상) 벽 3초에 걸쳐 오파시티 감소 후 No Collision
                (bind (_direction `_새_트랙_0`) (`Timeline|타임라인`)
                  (:`Update`
                    (`MaterialInstanceDynamic.SetScalarParameterValue` (`self.Wall_Dynamic`) "Opacity" `_새_트랙_0`))
                  (:`Finished`
                    (`PrimitiveComponent.SetCollisionEnabled` (`self.Wall_Cube`) "NoCollision")))
                (else
                  (`MaterialInstanceDynamic.SetScalarParameterValue` (`self.DynamicColor`) "B" 0.1)
                  ;[1 1 1] 제한 시간 증가 핸디캡
                  (set `self.Limit` (+ (`self.Limit`) 0.5))
                  (`self.K2_DestroyActor` _returnvalue_2)
                  (`self.K2_DestroyActor` _returnvalue)
                  (set `self.1/4Cleared` false)
                  (set `self.1/4bool` false)
                  (set `self.HalfCleared` false)
                  (set `self.Halfbool` false)
                  (set `self.3/4Cleared` false)
                  (set `self.3/4bool` false)
                  (if (and (`KismetSystemLibrary.IsValid` (stale `self.ReceiveActorBeginOverlap` _returnvalue_9)) (`KismetSystemLibrary.IsValid` (stale `self.ReceiveActorBeginOverlap` _returnvalue_10)))
                    (`self.K2_DestroyActor` (stale `self.ReceiveActorBeginOverlap` _returnvalue_10))
                    (`self.K2_DestroyActor` (stale `self.ReceiveActorBeginOverlap` _returnvalue_9))
                    (if (and (`KismetSystemLibrary.IsValid` (stale `self.ReceiveActorBeginOverlap` _returnvalue_7)) (`KismetSystemLibrary.IsValid` (stale `self.ReceiveActorBeginOverlap` _returnvalue_8)))
                      (`self.K2_DestroyActor` (stale `self.ReceiveActorBeginOverlap` _returnvalue_7))
                      (`self.K2_DestroyActor` (stale `self.ReceiveActorBeginOverlap` _returnvalue_8))
                      (if (and (`KismetSystemLibrary.IsValid` (stale `self.ReceiveActorBeginOverlap` _returnvalue_5)) (`KismetSystemLibrary.IsValid` (stale `self.ReceiveActorBeginOverlap` _returnvalue_6)))
                        (`self.K2_DestroyActor` (stale `self.ReceiveActorBeginOverlap` _returnvalue_5))
                        (`self.K2_DestroyActor` (stale `self.ReceiveActorBeginOverlap` _returnvalue_6))))))))
            (else
              (`KismetSystemLibrary.K2_SetTimerDelegate` (delegate `Volume_Manage`) 0.1)
              (if (`self.1/4bool`)
                (if (`self.Halfbool`)
                  (if (`self.3/4bool`)
                    _
                    (elif (`self.3/4Cleared`)
                      ;[1 1 1] 2번째 과녁 2개 생성
                      (`|ExecutionSequence`
                        (:`then_0`
                          (bind _returnvalue_5 (`|SpawnActorFromClass` "/Game/Blueprints/Objects/Target/BP_TargetMoving.BP_TargetMoving_C" (`KismetMathLibrary.MakeTransform` (990.0 -4000.0 500.0) (struct :`Yaw` 90.0)) "Undefined" "MultiplyWithRoot" null (990.0 -4000.0 500.0) (990.0 -2600.0 220.0) false null)))
                        (:`then_1`
                          (bind _returnvalue_6 (`|SpawnActorFromClass` "/Game/Blueprints/Objects/Target/BP_TargetRoundMoving.BP_TargetRoundMoving_C" (`KismetMathLibrary.MakeTransform` (690.0 -2550.0 360.0) (struct :`Yaw` 90.0)) "Undefined" "MultiplyWithRoot" null (690.0 -2550.0 360.0) null))
                          (set `self.3/4bool` true)
                          (`GameplayStatics.PlaySoundAtLocation` "/Game/Blueprints/Objects/Map_Objects/Bell_Sound.Bell_Sound" (990.0 -3445.0 200.0) (struct) 1.0 1.5 0.0 "/Game/Blueprints/Objects/Map_Objects/Bell_Attenuation.Bell_Attenuation" null null null)))))
                  (elif (`self.HalfCleared`)
                    ;[1 1 1] 3번째 과녁 2개 생성
                    (`|ExecutionSequence`
                      (:`then_0`
                        (bind _returnvalue_7 (`|SpawnActorFromClass` "/Game/Blueprints/Objects/Target/BP_TargetMoving.BP_TargetMoving_C" (`KismetMathLibrary.MakeTransform` (-1390.0 -3850.0 70.0) (struct :`Yaw` -90.0)) "Undefined" "MultiplyWithRoot" null (-1390.0 -3850.0 70.0) (-1390.0 -3850.0 580.0) false null)))
                      (:`then_1`
                        (bind _returnvalue_8 (`|SpawnActorFromClass` "/Game/Blueprints/Objects/Target/BP_TargetMoving.BP_TargetMoving_C" (`KismetMathLibrary.MakeTransform` (-1130.0 -3080.0 580.0) (struct :`Yaw` -90.0)) "Undefined" "MultiplyWithRoot" null (-1130.0 -3080.0 580.0) (-1130.0 -3080.0 70.0) false null))
                        (set `self.Halfbool` true)
                        (`GameplayStatics.PlaySoundAtLocation` "/Game/Blueprints/Objects/Map_Objects/Bell_Sound.Bell_Sound" (-1660.0 -3445.0 200.0) (struct) 1.0 1.5 0.0 "/Game/Blueprints/Objects/Map_Objects/Bell_Attenuation.Bell_Attenuation" null null null)))))
                (elif (`self.1/4Cleared`)
                  ;[1 1 1] 2번째 과녁 2개 생성
                  (`|ExecutionSequence`
                    (:`then_0`
                      (bind _returnvalue_9 (`|SpawnActorFromClass` "/Game/Blueprints/Objects/Target/BP_TargetMoving.BP_TargetMoving_C" (`KismetMathLibrary.MakeTransform` (990.0 -2600.0 220.0) (struct :`Yaw` 90.0)) "Undefined" "MultiplyWithRoot" null (990.0 -2600.0 220.0) (990.0 -4000.0 500.0) true null)))
                    (:`then_1`
                      (bind _returnvalue_10 (`|SpawnActorFromClass` "/Game/Blueprints/Objects/Target/BP_TargetFracture.BP_TargetFracture_C" (`KismetMathLibrary.MakeTransform` (990.0 -4490.0 440.0) (struct :`Yaw` -90.0)) "Undefined" "MultiplyWithRoot" null null))
                      (set `self.1/4bool` true)
                      (`GameplayStatics.PlaySoundAtLocation` "/Game/Blueprints/Objects/Map_Objects/Bell_Sound.Bell_Sound" (990.0 -3445.0 200.0) (struct) 1.0 1.5 0.0 "/Game/Blueprints/Objects/Map_Objects/Bell_Attenuation.Bell_Attenuation" null null null))))))))))))

(event `Volume_Manage`
  (`AudioComponent.SetVolumeMultiplier` (stale `self.ReceiveActorBeginOverlap` _returnvalue_4) (`KismetMathLibrary.FClamp` (/ (/ (`/Game/Blueprints/Objects/Map_Objects/BP_Timer_Sample.Limit` (stale `self.ReceiveActorBeginOverlap` _output_get)) (`/Game/Blueprints/Objects/Map_Objects/BP_Timer_Sample.Remain_Time` (stale `self.ReceiveActorBeginOverlap` _output_get))) 3.0) 0.0 4.0))
  (if (`self.1/4Cleared`)
    (if (`self.HalfCleared`)
      (if (`self.3/4Cleared`)
        (bind _output_get (set `self.IsCleared` (and (`/Game/Blueprints/Objects/Target/BP_TargetMoving.Clear` (stale `self.ReceiveActorBeginOverlap` _returnvalue_5)) (`/Game/Blueprints/Objects/Target/BP_TargetRoundMoving.Clear` (stale `self.ReceiveActorBeginOverlap` _returnvalue_6)))))
        (goto _label)
        (else
          (set `self.3/4Cleared` (and (`/Game/Blueprints/Objects/Target/BP_TargetMoving.Clear` (stale `self.ReceiveActorBeginOverlap` _returnvalue_7)) (`/Game/Blueprints/Objects/Target/BP_TargetMoving.Clear` (stale `self.ReceiveActorBeginOverlap` _returnvalue_8))))
          (goto _label)))
      (else
        (set `self.HalfCleared` (and (`/Game/Blueprints/Objects/Target/BP_TargetMoving.Clear` (stale `self.ReceiveActorBeginOverlap` _returnvalue_9)) (`/Game/Blueprints/Objects/Target/BP_TargetFracture.Clear` (stale `self.ReceiveActorBeginOverlap` _returnvalue_10))))
        (goto _label)))
    (else
      (set `self.1/4Cleared` (and (`/Game/Blueprints/Objects/Target/BP_TargetMoving.Clear` (stale `self.ReceiveActorBeginOverlap` _returnvalue)) (`/Game/Blueprints/Objects/Target/BP_TargetFracture.Clear` (stale `self.ReceiveActorBeginOverlap` _returnvalue_2))))
      (goto _label))))

(fn `UserConstructionScript`)