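; Combat puzzle button that, when the player character overlaps it, starts a timed target-shattering challenge to open an electric wall.
; It spawns two successive waves of four BP_TargetFracture actors at fixed locations and shows a countdown widget.
; A self-rearming 0.1-second timer polls target Clear flags and raises timer audio volume as time runs out.
; Success fades the wall via Timeline and disables its collision, while failure resets and slightly extends the time limit.
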(event `self.ReceiveBeginPlay`
  (bind _returnvalue (`PrimitiveComponent.CreateDynamicMaterialInstance` (`self.Cube`) 0 "/Game/Blueprints/Objects/Map_Objects/Button_Sample_material.Button_Sample_material" "None"))
  (bind _output_get (set `self.DynamicColor` _returnvalue))
  (`PrimitiveComponent.SetMaterial` (`self.Cube`) 0 _output_get)
  (`MaterialInstanceDynamic.SetScalarParameterValue` _output_get "B" 0.5)
  ;[1 1 1] 벽 오파시티 조정 밑작업
  (bind _returnvalue_2 (`PrimitiveComponent.CreateDynamicMaterialInstance` (`self.Wall_Cube`) 0 "/Game/Blueprints/Objects/Map_Objects/EletroWall_Sample.EletroWall_Sample" "None"))
  (bind _output_get_2 (set `self.Wall_Dynamic` _returnvalue_2))
  (`PrimitiveComponent.SetMaterial` (`self.Wall_Cube`) 0 _output_get_2))

(event `self.ReceiveActorBeginOverlap`
  (params (OtherActor :type "Actor Object Reference"))
  (bind _returnvalue (`KismetMathLibrary.MakeTransform` (-4195.0 -2275.0 170.0) (struct :`Yaw` 90.0)))
  (bind _returnvalue_2 (`KismetMathLibrary.MakeTransform` (-4195.0 -2675.0 370.0) (struct :`Yaw` 90.0)))
  (bind _limit (`self.Limit`))
  (cast `/Game/ThirdPerson/Blueprints/BP_ThirdPersonCharacter` OtherActor)
  (if (`self.IsCleared`)
    _
    (elif (not (`self.OnProgress`))
      (`MaterialInstanceDynamic.SetScalarParameterValue` (`self.DynamicColor`) "B" 0.0)
      ;[1 1 1] 과녁 4개 생성
      (`|ExecutionSequence`
        (:`then_0`
          (bind _returnvalue_3 (`|SpawnActorFromClass` "/Game/Blueprints/Objects/Target/BP_TargetFracture.BP_TargetFracture_C" (`KismetMathLibrary.MakeTransform` (-4195.0 -2275.0 370.0) (struct :`Yaw` 90.0)) "Undefined" "MultiplyWithRoot" null null)))
        (:`then_1`
          (bind _returnvalue_4 (`|SpawnActorFromClass` "/Game/Blueprints/Objects/Target/BP_TargetFracture.BP_TargetFracture_C" _returnvalue_2 "Undefined" "MultiplyWithRoot" null null)))
        (:`then_2`
          (bind _returnvalue_5 (`|SpawnActorFromClass` "/Game/Blueprints/Objects/Target/BP_TargetFracture.BP_TargetFracture_C" (`KismetMathLibrary.MakeTransform` (-4195.0 -2475.0 570.0) (struct :`Yaw` 90.0)) "Undefined" "MultiplyWithRoot" null null)))
        (:`then_3`
          (bind _returnvalue_6 (`|SpawnActorFromClass` "/Game/Blueprints/Objects/Target/BP_TargetFracture.BP_TargetFracture_C" (`KismetMathLibrary.MakeTransform` (-4195.0 -2475.0 170.0) (struct :`Yaw` 90.0)) "Undefined" "MultiplyWithRoot" null null))
          (`GameplayStatics.PlaySoundAtLocation` "/Game/Blueprints/Objects/Map_Objects/Bell_Sound.Bell_Sound" (.location _returnvalue_2) (struct) 1.0 1.5 0.0 "/Game/Blueprints/Objects/Map_Objects/Bell_Attenuation.Bell_Attenuation" null null null)
          ;[1 1 1] 위젯 및 타이머 소리 재생
          (bind _returnvalue_7 (`|CreateWidget` "/Game/Blueprints/Objects/Map_Objects/BP_Timer_Sample.BP_Timer_Sample_C" null _limit _limit))
          (bind _output_get (set `self.BP_Widget` _returnvalue_7))
          (`UserWidget.AddToViewport` _output_get 0)
          (set `self.OnProgress` true)
          (bind _returnvalue_8 (`AddComponent|NODE_AddAudioComponent-5`))
          (`SceneComponent.K2_SetWorldLocation` _returnvalue_8 (0.0 0.0 0.0) false false)
          (if (or (>= 0.0 (`/Game/Blueprints/Objects/Map_Objects/BP_Timer_Sample.Remain_Time` _output_get)) (stale `Volume_Manage` _output_get)) :!label _label
            (`AudioComponent.Stop` _returnvalue_8)
            (if (`KismetSystemLibrary.IsValid` _returnvalue_7)
              (`Widget.RemoveFromParent` _returnvalue_7)
              (set `self.OnProgress` false)
              (if (`self.IsCleared`)
                ;[1 1 1] (클리어 보상) 벽 3초에 걸쳐 오파시티 감소 후 No Collision
                (bind (_direction `_새_트랙_0`) (`Timeline|타임라인`)
                  (:`Update`
                    (`MaterialInstanceDynamic.SetScalarParameterValue` (`self.Wall_Dynamic`) "Opacity" `_새_트랙_0`))
                  (:`Finished`
                    (`PrimitiveComponent.SetCollisionEnabled` (`self.Wall_Cube`) "NoCollision")))
                (else
                  (`MaterialInstanceDynamic.SetScalarParameterValue` (`self.DynamicColor`) "B" 0.5)
                  ;[1 1 1] 제한 시간 증가 핸디캡
                  (set `self.Limit` (+ (`self.Limit`) 0.25))
                  (`self.K2_DestroyActor` _returnvalue_4)
                  (`self.K2_DestroyActor` _returnvalue_3)
                  (`self.K2_DestroyActor` _returnvalue_5)
                  (`self.K2_DestroyActor` _returnvalue_6)
                  (set `self.HalfCleared` false)
                  (set `self.Halfbool` false)
                  (if (and (`KismetSystemLibrary.IsValid` (stale `self.ReceiveActorBeginOverlap` _returnvalue_9)) (`KismetSystemLibrary.IsValid` (stale `self.ReceiveActorBeginOverlap` _returnvalue_10)) (`KismetSystemLibrary.IsValid` (stale `self.ReceiveActorBeginOverlap` _returnvalue_11)) (`KismetSystemLibrary.IsValid` (stale `self.ReceiveActorBeginOverlap` _returnvalue_12)))
                    (`self.K2_DestroyActor` (stale `self.ReceiveActorBeginOverlap` _returnvalue_9))
                    (`self.K2_DestroyActor` (stale `self.ReceiveActorBeginOverlap` _returnvalue_10))
                    (`self.K2_DestroyActor` (stale `self.ReceiveActorBeginOverlap` _returnvalue_11))
                    (`self.K2_DestroyActor` (stale `self.ReceiveActorBeginOverlap` _returnvalue_12))))))
            (else
              (`KismetSystemLibrary.K2_SetTimerDelegate` (delegate `Volume_Manage`) 0.1)
              (if (`self.Halfbool`)
                _
                (elif (`self.HalfCleared`)
                  ;[1 1 1] 2번째 과녁 4개 생성
                  (`|ExecutionSequence`
                    (:`then_0`
                      (bind _returnvalue_9 (`|SpawnActorFromClass` "/Game/Blueprints/Objects/Target/BP_TargetFracture.BP_TargetFracture_C" (`KismetMathLibrary.MakeTransform` (-4195.0 -2275.0 570.0) (struct :`Yaw` 90.0)) "Undefined" "MultiplyWithRoot" null null)))
                    (:`then_1`
                      (bind _returnvalue_10 (`|SpawnActorFromClass` "/Game/Blueprints/Objects/Target/BP_TargetFracture.BP_TargetFracture_C" (`KismetMathLibrary.MakeTransform` (-4195.0 -2675.0 170.0) (struct :`Yaw` 90.0)) "Undefined" "MultiplyWithRoot" null null)))
                    (:`then_2`
                      (bind _returnvalue_11 (`|SpawnActorFromClass` "/Game/Blueprints/Objects/Target/BP_TargetFracture.BP_TargetFracture_C" (`KismetMathLibrary.MakeTransform` (-4195.0 -2675.0 570.0) (struct :`Yaw` 90.0)) "Undefined" "MultiplyWithRoot" null null)))
                    (:`then_3`
                      (bind _returnvalue_12 (`|SpawnActorFromClass` "/Game/Blueprints/Objects/Target/BP_TargetFracture.BP_TargetFracture_C" _returnvalue "Undefined" "MultiplyWithRoot" null null))
                      (set `self.Halfbool` true)
                      (`GameplayStatics.PlaySoundAtLocation` null (.location _returnvalue) (struct) 1.0 1.5 0.0 null null null null))))))))))))

(event `Volume_Manage`
  (`AudioComponent.SetVolumeMultiplier` (stale `self.ReceiveActorBeginOverlap` _returnvalue_8) (`KismetMathLibrary.FClamp` (/ (/ (`/Game/Blueprints/Objects/Map_Objects/BP_Timer_Sample.Limit` (stale `self.ReceiveActorBeginOverlap` _output_get)) (`/Game/Blueprints/Objects/Map_Objects/BP_Timer_Sample.Remain_Time` (stale `self.ReceiveActorBeginOverlap` _output_get))) 2.0) 0.0 4.0))
  (if (`self.HalfCleared`)
    (bind _output_get (set `self.IsCleared` (and (`/Game/Blueprints/Objects/Target/BP_TargetFracture.Clear` (stale `self.ReceiveActorBeginOverlap` _returnvalue_9)) (`/Game/Blueprints/Objects/Target/BP_TargetFracture.Clear` (stale `self.ReceiveActorBeginOverlap` _returnvalue_10)) (`/Game/Blueprints/Objects/Target/BP_TargetFracture.Clear` (stale `self.ReceiveActorBeginOverlap` _returnvalue_11)) (`/Game/Blueprints/Objects/Target/BP_TargetFracture.Clear` (stale `self.ReceiveActorBeginOverlap` _returnvalue_12)))))
    (goto _label)
    (else
      (set `self.HalfCleared` (and (`/Game/Blueprints/Objects/Target/BP_TargetFracture.Clear` (stale `self.ReceiveActorBeginOverlap` _returnvalue_3)) (`/Game/Blueprints/Objects/Target/BP_TargetFracture.Clear` (stale `self.ReceiveActorBeginOverlap` _returnvalue_4)) (`/Game/Blueprints/Objects/Target/BP_TargetFracture.Clear` (stale `self.ReceiveActorBeginOverlap` _returnvalue_5)) (`/Game/Blueprints/Objects/Target/BP_TargetFracture.Clear` (stale `self.ReceiveActorBeginOverlap` _returnvalue_6))))
      (goto _label))))

(fn `UserConstructionScript`)