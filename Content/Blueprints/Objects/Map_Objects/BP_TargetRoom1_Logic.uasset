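; Map object logic for target room 1: clearing its three BP_TargetFracture targets opens an electric wall as the reward.
; On BeginPlay it gives WallCube a dynamic material and binds each target's clear event to a shared check.
; When that check finds all three targets cleared, a timeline fades the wall's Opacity parameter, then disables its collision.
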(event `self.ReceiveBeginPlay`
  ;[1 1 1] 벽 오파시티 조정 밑작업
  (bind _returnvalue (`PrimitiveComponent.CreateDynamicMaterialInstance` (`self.Wall_Cube`) 0 "/Game/Blueprints/Objects/Map_Objects/EletroWall_Sample.EletroWall_Sample" "None"))
  (bind _output_get (set `self.Wall_Dynamic` _returnvalue))
  (`PrimitiveComponent.SetMaterial` (`self.Wall_Cube`) 0 _output_get)
  (for _array_element (`|MakeArray` (`self.L_Target`) (`self.M_Target`) (`self.R_Target`))
    (bind _asbp_target_fracture (cast `/Game/Blueprints/Objects/Target/BP_TargetFracture` _array_element))
    (add `/Game/Blueprints/Objects/Target/BP_TargetFracture.Target1_Clear` _asbp_target_fracture (delegate `TargetRoom1_Clear`))))

(event `TargetRoom1_Clear`
  (for _array_element (`|MakeArray` (`self.L_Target`) (`self.M_Target`) (`self.R_Target`))
    (bind _asbp_target_fracture (cast `/Game/Blueprints/Objects/Target/BP_TargetFracture` _array_element))
    (if (not (`/Game/Blueprints/Objects/Target/BP_TargetFracture.Clear` _asbp_target_fracture))
      (bind _output_get (set `self.All_Clear` false))))
  (if _output_get
    ;[1 1 1] (클리어 보상) 벽 3초에 걸쳐 오파시티 감소 후 No Collision
    (bind (_direction `_새_트랙_0`) (`Timeline|타임라인`)
      (:`Update`
        (`MaterialInstanceDynamic.SetScalarParameterValue` (`self.Wall_Dynamic`) "Opacity" `_새_트랙_0`))
      (:`Finished`
        (`PrimitiveComponent.SetCollisionEnabled` (`self.Wall_Cube`) "NoCollision")))
    (else
      (set `self.All_Clear` true))))

(fn `UserConstructionScript`)