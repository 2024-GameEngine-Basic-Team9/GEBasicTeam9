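; BP_Grenade is a grenade that, once activated, beeps a set number of times, then explodes.
; Tick drives the beep timer, then plays explosion effects and briefly enables overlap events on its collision.
; Sphere overlaps damage nearby BP_Boss and BP_Zombie actors, bosses far more heavily, before a delayed self-destroy.
; The StunUpgrade function sets a flag that adds a spark effect and stuns bosses hit by the blast.
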(event `self.ReceiveBeginPlay`
  (`ActorComponent.SetActive` (`self.Spark`) false false))

(event `ActivateGrenade_Event`
  (set `self.Activate` true))

(event `self.ReceiveTick`
  (params (DeltaSeconds :type "Float (single-precision)"))
  (bind _array (`|MakeArray` "ObjectTypeQuery2" "ObjectTypeQuery7" :!type "EObjectTypeQuery Enum"))
  (bind _returnvalue (`SceneComponent.K2_GetComponentLocation` (`self.GrenadeBody`)))
  (if (`self.Activate`)
    (bind _output_get (set `self.BeepTimer` (+ (`self.BeepTimer`) DeltaSeconds)))
    (if (`self.BeepFlag`)
      (if (>= _output_get (`self.BeepPeriod`))
        (set `self.BeepTimer` 0.0)
        (`GameplayStatics.PlaySoundAtLocation` "/Game/Resources/Sound/beep-104060.beep-104060" (`SceneComponent.K2_GetComponentLocation` (`self.GrenadeBody`)) (struct) 1.0 1.0 0.0 null null null null)
        (bind _result (`/Engine/EditorBlueprintResources/StandardMacros.IncrementInt` (`self.Counter`))
          (:`  `
            (if (== _result (`self.MaxCount`))
              (set `self.BeepFlag` false)))))
      (elif (>= _output_get (`self.BeepPeriod`))
        (set `self.Activate` false)
        (`GameplayStatics.PlaySoundAtLocation` "/Game/Resources/Sound/medium-explosion-40472.medium-explosion-40472" (`SceneComponent.K2_GetComponentLocation` (`self.GrenadeBody`)) (struct) 1.0 1.0 0.0 null null null null)
        (`ActorComponent.Activate` (`self.Explosion`) false)
        (set `PrimitiveComponent.bGenerateOverlapEvents` true (`self.Collision`))
        (`KismetSystemLibrary.Delay` 0.3)
        (set `PrimitiveComponent.bGenerateOverlapEvents` false (`self.Collision`))
        (if (`self.StunUpgraded`)
          (`ActorComponent.SetActive` (`self.Spark`) true false))
        (`|ExecutionSequence`
          (:`then_0`
            (bind _outactors (`KismetSystemLibrary.SphereOverlapActors` _returnvalue 500.0 _array "/Game/Blueprints/Characters/BP_Boss.BP_Boss_C"))
            (for _array_element _outactors
              (bind _asbp_boss (cast `/Game/Blueprints/Characters/BP_Boss` _array_element))
              (`/Game/Blueprints/Characters/BP_Boss.OnBossHit` _asbp_boss 2000.0)
              (if (`self.StunUpgraded`)
                (`/Game/Blueprints/Characters/BP_Boss.OnStun` _asbp_boss)
                (`/Game/Blueprints/Characters/BP_Boss.Stun_Event` _asbp_boss))))
          (:`then_1`
            (bind _outactors_2 (`KismetSystemLibrary.SphereOverlapActors` _returnvalue 500.0 _array "/Game/Blueprints/Characters/BP_Zombie.BP_Zombie_C"))
            (for _array_element_2 _outactors_2
              (bind _asbp_zombie (cast `/Game/Blueprints/Characters/BP_Zombie` _array_element_2))
              (`/Game/Blueprints/Characters/BP_Zombie.OnEnemyHit` _asbp_zombie 200.0)))
          (:`then_2`
            (`KismetSystemLibrary.Delay` 3.7)
            (`self.K2_DestroyActor`)))))))

(fn `StunUpgrade`
  (set `self.StunUpgraded` true))

(fn `UserConstructionScript`)