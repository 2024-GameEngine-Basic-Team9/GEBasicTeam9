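; BP_TargetRoundMoving is a hittable target that moves along a circular path and shatters when hit.
; TargetMove plays a timeline whose track drives sine and cosine offsets, placing the actor on a vertical Y-Z circle around Center at Radius.
; The first hit sets the Clear guard, destroys the intact TargetFull component, spawns BP_TargetFracture with yaw turned half a turn, and triggers its fracture.
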(event `TargetMove`
  (bind (_direction `_새_트랙_0`) (`Timeline|타임라인`)
    (:`Update`
      (bind _returnvalue (* `_새_트랙_0` 6.3))
      (`self.K2_SetActorLocation` (`KismetMathLibrary.MakeVector` (.x (`self.Center`)) (+ (* (`KismetMathLibrary.Cos` _returnvalue) (`self.Radius`)) (.y (`self.Center`))) (+ (* (`KismetMathLibrary.Sin` _returnvalue) (`self.Radius`)) (.z (`self.Center`))))))))

(fn `On TargetMoving Hit`
  (if (not (`self.Clear`))
    (set `self.Clear` true)
    (bind _output_get (set `self.SpawnTransform` (`KismetMathLibrary.MakeTransform` (.location (`self.GetTransform`)) (`KismetMathLibrary.MakeRotator` (.roll (.rotation (`self.GetTransform`))) (.pitch (.rotation (`self.GetTransform`))) (+ (.yaw (.rotation (`self.GetTransform`))) 180.0)))))
    (`ActorComponent.K2_DestroyComponent` (`self.TargetFull`))
    (bind _returnvalue (`|SpawnActorFromClass` "/Game/Blueprints/Objects/Target/BP_TargetFracture.BP_TargetFracture_C" _output_get "AlwaysSpawn" "MultiplyWithRoot" null null))
    (`/Game/Blueprints/Objects/Target/BP_TargetFracture.On TargetFracture Hit` _returnvalue)
    (set `self.Clear` true)))

(fn `UserConstructionScript`)