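; BP_TargetMoving is a target that moves between two points and breaks apart when hit.
; TargetMove plays a timeline that lerps between Point1 and Point2, with the Track flag choosing the curve, and applies swept offsets.
; On a hit, guarded by Clear to run once, it destroys the TargetFull component and spawns BP_TargetFracture yawed 180 degrees, then triggers its fracture hit.
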(event `TargetMove`
  (bind (_direction `_새_트랙_0` `_새_트랙_1`) (`Timeline|타임라인`)
    (:`Update`
      (if (`self.Track`)
        (`self.K2_AddActorWorldOffset` (- (`KismetMathLibrary.VLerp` (`self.Point1`) (`self.Point2`) `_새_트랙_0`) (`self.K2_GetActorLocation`)) true)
        (else
          (`self.K2_AddActorWorldOffset` (- (`KismetMathLibrary.VLerp` (`self.Point1`) (`self.Point2`) `_새_트랙_1`) (`self.K2_GetActorLocation`)) true))))))

(fn `On TargetMoving Hit`
  (if (not (`self.Clear`))
    (set `self.Clear` true)
    (bind _output_get (set `self.SpawnTransform` (`KismetMathLibrary.MakeTransform` (.location (`self.GetTransform`)) (`KismetMathLibrary.MakeRotator` (.roll (.rotation (`self.GetTransform`))) (.pitch (.rotation (`self.GetTransform`))) (+ (.yaw (.rotation (`self.GetTransform`))) 180.0)))))
    (`ActorComponent.K2_DestroyComponent` (`self.TargetFull`))
    (bind _returnvalue (`|SpawnActorFromClass` "/Game/Blueprints/Objects/Target/BP_TargetFracture.BP_TargetFracture_C" _output_get "AlwaysSpawn" "MultiplyWithRoot" null null))
    (`/Game/Blueprints/Objects/Target/BP_TargetFracture.On TargetFracture Hit` _returnvalue)
    (set `self.Clear` true)))

(fn `UserConstructionScript`)