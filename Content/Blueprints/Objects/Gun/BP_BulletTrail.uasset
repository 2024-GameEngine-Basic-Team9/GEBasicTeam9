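; BP_BulletTrail is a short-lived gun effect actor that draws a bullet trail to a given end point.
; Fire stores the start and end positions and enables movement, then Tick teleports the NSTrailEffect component straight to the end position rather than interpolating.
; The actor destroys itself after a brief delay from BeginPlay, while the stored start position and the arrival check in Tick drive no further logic.
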(event `self.ReceiveBeginPlay`
  (`KismetSystemLibrary.Delay` 0.1)
  (`self.K2_DestroyActor`))

(event `self.ReceiveTick`
  (params (DeltaSeconds :type "Float (single-precision)"))
  (if (`self.Move`)
    (`SceneComponent.K2_SetWorldLocation` (`self.NS_TrailEffect`) (`self.EndPosition`) false true)
    (if (== (`SceneComponent.K2_GetComponentLocation` (`self.NS_TrailEffect`)) (`self.EndPosition`) :`ErrorTolerance` 100.0)
      _)))

(fn `Fire`
  (params (EndPosition :type "Vector Structure"))
  (set `self.Move` true)
  (set `self.EndPosition` EndPosition)
  (set `self.StartPosition` (`SceneComponent.K2_GetComponentLocation` (`self.NS_TrailEffect`))))

(fn `UserConstructionScript`)