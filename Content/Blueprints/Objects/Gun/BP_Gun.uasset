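; Gun actor with four decorative emissive rings that flash when its fire effect is triggered.
; BeginPlay creates a dynamic material instance of MT_Emissive for each ring.
; FireEffect stores the supplied brightness and momentarily zeroes the rings' Brightness parameter.
; Tick pushes the stored brightness to all four materials, decaying it linearly at a fast fixed rate back to a baseline glow.
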(event `self.ReceiveTick`
  (params (DeltaSeconds :type "Float (single-precision)"))
  (bind _brightness (`self.Brightness`))
  (`|ExecutionSequence`
    (:`then_0`
      (if (> (`self.Brightness`) 1.0)
        (set `self.Brightness` (- (`self.Brightness`) (* DeltaSeconds 500.0)))
        (else
          (set `self.Brightness` 1.0))))
    (:`then_1`
      (`MaterialInstanceDynamic.SetScalarParameterValue` (`self.DecoRing1Material`) "Brightness" _brightness)
      (`MaterialInstanceDynamic.SetScalarParameterValue` (`self.DecoRing2Material`) "Brightness" _brightness)
      (`MaterialInstanceDynamic.SetScalarParameterValue` (`self.DecoRing3Material`) "Brightness" _brightness)
      (`MaterialInstanceDynamic.SetScalarParameterValue` (`self.DecoRing4Material`) "Brightness" _brightness))))

(event `self.ReceiveBeginPlay`
  (bind _returnvalue (`PrimitiveComponent.CreateDynamicMaterialInstance` (`self.DecoRing1`) 0 "/Game/Resources/Materials/MT_Emissive.MT_Emissive" "None"))
  (set `self.DecoRing1Material` _returnvalue)
  (bind _returnvalue_2 (`PrimitiveComponent.CreateDynamicMaterialInstance` (`self.DecoRing2`) 0 "/Game/Resources/Materials/MT_Emissive.MT_Emissive" "None"))
  (set `self.DecoRing2Material` _returnvalue_2)
  (bind _returnvalue_3 (`PrimitiveComponent.CreateDynamicMaterialInstance` (`self.DecoRing3`) 0 "/Game/Resources/Materials/MT_Emissive.MT_Emissive" "None"))
  (set `self.DecoRing3Material` _returnvalue_3)
  (bind _returnvalue_4 (`PrimitiveComponent.CreateDynamicMaterialInstance` (`self.DecoRing4`) 0 "/Game/Resources/Materials/MT_Emissive.MT_Emissive" "None"))
  (set `self.DecoRing4Material` _returnvalue_4))

(fn `FireEffect`
  (params (RingBrightness :type "Float (double-precision)"))
  (set `self.Brightness` RingBrightness)
  (`MaterialInstanceDynamic.SetScalarParameterValue` (`self.DecoRing1Material`) "Brightness" 0.0)
  (`MaterialInstanceDynamic.SetScalarParameterValue` (`self.DecoRing2Material`) "Brightness" 0.0)
  (`MaterialInstanceDynamic.SetScalarParameterValue` (`self.DecoRing3Material`) "Brightness" 0.0)
  (`MaterialInstanceDynamic.SetScalarParameterValue` (`self.DecoRing4Material`) "Brightness" 0.0))

(fn `UserConstructionScript`)