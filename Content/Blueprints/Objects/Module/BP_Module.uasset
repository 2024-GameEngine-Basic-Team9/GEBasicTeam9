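; BP_Module is a pickup actor that activates a module when the player's character touches it.
; On BeginPlay it caches the first player's BP_PlayerStateCustom and BP_ThirdPersonCharacter.
; When that character overlaps it, it passes its RoomIndex to SetModule on the player state, plays a pickup sound at its location and destroys itself.
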(event `self.ReceiveBeginPlay`
  (bind _asbp_player_state_custom (cast `/Game/Blueprints/BP_PlayerStateCustom` (`GameplayStatics.GetPlayerState` 0)))
  (set `self.BP Player State Custom` _asbp_player_state_custom)
  (bind _asbp_third_person_character (cast `/Game/ThirdPerson/Blueprints/BP_ThirdPersonCharacter` (`GameplayStatics.GetPlayerPawn` 0)))
  (set `self.BP Third Person Character` _asbp_third_person_character))

(event `self.ReceiveActorBeginOverlap`
  (params (OtherActor :type "Actor Object Reference"))
  ;[1 1 1] When overlapping, module activation
  (if (== OtherActor (`self.BP Third Person Character`))
    (`/Game/Blueprints/BP_PlayerStateCustom.SetModule` (`self.BP Player State Custom`) (`self.RoomIndex`))
    (`GameplayStatics.PlaySoundAtLocation` "/Game/Resources/Sound/Puzzle/item_get.item_get" (`SceneComponent.K2_GetComponentLocation` (`self.DefaultSceneRoot`)) (struct) 1.3 1.0 0.0 null null null null)
    (`self.K2_DestroyActor`)))

(fn `UserConstructionScript`)