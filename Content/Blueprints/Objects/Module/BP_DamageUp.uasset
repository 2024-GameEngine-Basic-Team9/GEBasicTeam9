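; A pickup module that raises the player character's damage when touched.
; On BeginPlay it caches the player character and the custom HUD.
; When the player overlaps its sphere, it applies a damage upgrade, plays a pickup sound, shows an info message on the main UI and destroys itself.
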(event `self.ReceiveBeginPlay`
  (bind _asbp_third_person_character (cast `/Game/ThirdPerson/Blueprints/BP_ThirdPersonCharacter` (`GameplayStatics.GetPlayerPawn` 0)))
  (set `self.As BP Third Person Character` _asbp_third_person_character)
  (bind _asbp_hudcustom (cast `/Game/UI/BP_HUDCustom` (`PlayerController.GetHUD` (`GameplayStatics.GetPlayerController` 0))))
  (set `self.HUDCustom` _asbp_hudcustom))

(event `self.Sphere.OnComponentBeginOverlap`
  (params (OverlappedComponent :type "PrimitiveComponent Object Reference") (OtherActor :type "Actor Object Reference") (OtherComp :type "PrimitiveComponent Object Reference") (OtherBodyIndex :type Integer) (bFromSweep :type Boolean) (SweepResult :type "HitResult Structure (by ref)"))
  (bind _as_bp_third_person_character (`self.As BP Third Person Character`))
  (if (== OtherActor _as_bp_third_person_character)
    (`/Game/ThirdPerson/Blueprints/BP_ThirdPersonCharacter.Upgrade_AddDamage` _as_bp_third_person_character 3.5)
    (`GameplayStatics.PlaySoundAtLocation` "/Game/Resources/Sound/Puzzle/item_get.item_get" (`SceneComponent.K2_GetComponentLocation` (`self.Scene`)) (struct) 1.3 1.0 0.0 null null null null)
    (`/Game/UI/UI_MainUI.SetInfoText` (`/Game/UI/BP_HUDCustom.MainUI` (`self.HUDCustom`)) "Damage Increased")
    (`self.K2_DestroyActor`)))

(fn `UserConstructionScript`)