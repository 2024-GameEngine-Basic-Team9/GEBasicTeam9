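; BP_CardKey is a key card pickup that unlocks a door for the player.
; It starts hidden with collision off, then becomes visible and query-collidable when ControlRef fires its Cleared dispatcher.
; When the player pawn overlaps it, it sets its DoorIndex entry in the IsDoorOpen array on BP_PlayerStateCustom and destroys itself.
; It is meant as a base class, with child Blueprints overriding DoorIndex.
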(event `self.ReceiveBeginPlay`
  ;[1 1 1] Set it not visible
  (`SceneComponent.SetVisibility` (`self.DefaultSceneRoot`) false true)
  (`PrimitiveComponent.SetCollisionEnabled` (`self.Collision`) "NoCollision")
  (add `/Game/Blueprints/BP_PuzzleRoomControl.Cleared` (`self.ControlRef`) (delegate `Appear`)))

(event `Appear`
  ;[1 1 1] When cleared, set it visible (need to event dispatcher)
  (`SceneComponent.SetVisibility` (`self.DefaultSceneRoot`) true true)
  (`PrimitiveComponent.SetCollisionEnabled` (`self.Collision`) "QueryOnly"))

(event `self.ReceiveActorBeginOverlap`
  (params (OtherActor :type "Actor Object Reference"))
  ;[1 1 1] 상속 후 DoorIndex 값 수정하여 사용
  (`self.DoorOpen` OtherActor))

(fn `DoorOpen`
  (params (Overlapped_Object :type "Actor Object Reference"))
  (if (== Overlapped_Object (`GameplayStatics.GetPlayerPawn` 0))
    (bind _asbp_player_state_custom (cast `/Game/Blueprints/BP_PlayerStateCustom` (`GameplayStatics.GetPlayerState` 0)))
    (`KismetArrayLibrary.Array_Set` (`/Game/Blueprints/BP_PlayerStateCustom.IsDoorOpen` _asbp_player_state_custom) (`self.DoorIndex`) true)
    (`self.K2_DestroyActor`)))

(fn `UserConstructionScript`)