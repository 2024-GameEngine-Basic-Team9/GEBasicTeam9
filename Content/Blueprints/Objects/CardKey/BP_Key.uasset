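; BP_Key is a spinning keycard pickup that unlocks a door by its DoorID when the player character touches its sphere.
; On BeginPlay it caches the custom PlayerState, third-person character and HUD.
; On overlap it sets that index in the PlayerState's IsDoorOpen array, plays a pickup sound, shows a numbered Training or Puzzle Room message and destroys itself.
; Tick slowly rotates the card mesh.
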(event `self.ReceiveBeginPlay`
  (bind _asbp_player_state_custom (cast `/Game/Blueprints/BP_PlayerStateCustom` (`GameplayStatics.GetPlayerState` 0)))
  (set `self.BP Player State Custom` _asbp_player_state_custom)
  (bind _asbp_third_person_character (cast `/Game/ThirdPerson/Blueprints/BP_ThirdPersonCharacter` (`GameplayStatics.GetPlayerPawn` 0)))
  (set `self.BP Third Person Character` _asbp_third_person_character)
  (bind _asbp_hudcustom (cast `/Game/UI/BP_HUDCustom` (`PlayerController.GetHUD` (`GameplayStatics.GetPlayerController` 0))))
  (set `self.HUDCustom` _asbp_hudcustom))

(event `self.Sphere.OnComponentBeginOverlap`
  (params (OverlappedComponent :type "PrimitiveComponent Object Reference") (OtherActor :type "Actor Object Reference") (OtherComp :type "PrimitiveComponent Object Reference") (OtherBodyIndex :type Integer) (bFromSweep :type Boolean) (SweepResult :type "HitResult Structure (by ref)"))
  (if (== OtherActor (`self.BP Third Person Character`))
    (`KismetArrayLibrary.Array_Set` (`/Game/Blueprints/BP_PlayerStateCustom.IsDoorOpen` (`self.BP Player State Custom`)) (`self.DoorID`) true)
    (`GameplayStatics.PlaySoundAtLocation` "/Game/Resources/Sound/Puzzle/item_get.item_get" (`SceneComponent.K2_GetComponentLocation` (`self.DefaultSceneRoot`)) (struct) 1.0 1.0 0.0 null null null null)
    (if (< (`self.DoorID`) 3)
      (bind _output_get (set `self.RoomName` "Collected Key For Training Room "))
      (`/Game/UI/UI_MainUI.SetInfoText` (`/Game/UI/BP_HUDCustom.MainUI` (`self.HUDCustom`)) (`KismetTextLibrary.Conv_StringToText` (`KismetStringLibrary.Concat_StrStr` (`KismetTextLibrary.Conv_TextToString` _output_get) (`KismetStringLibrary.Conv_IntToString` (+ (`self.DoorID`) 1)))))
      (`self.K2_DestroyActor`)
      (else
        (bind _output_get_2 (set `self.RoomName` "Collected Key For Puzzle Room "))
        (`/Game/UI/UI_MainUI.SetInfoText` (`/Game/UI/BP_HUDCustom.MainUI` (`self.HUDCustom`)) (`KismetTextLibrary.Conv_StringToText` (`KismetStringLibrary.Concat_StrStr` (`KismetTextLibrary.Conv_TextToString` _output_get_2) (`KismetStringLibrary.Conv_IntToString` (- (`self.DoorID`) 2)))))
        (`self.K2_DestroyActor`)))))

(event `self.ReceiveTick`
  (params (DeltaSeconds :type "Float (single-precision)"))
  (`SceneComponent.K2_AddWorldRotation` (`self.CardKey`) (* (struct :`Pitch` 1.0 :`Yaw` 1.0 :`Roll` 1.0) (* DeltaSeconds 14.0)) false false))

(fn `UserConstructionScript`)