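; BP_ZombieSpawner is a wave-based spawner that creates BP_Zombie actors at four arrow points.
; On BeginPlay it binds six wave events to activation dispatchers on BP_PlayerStateCustom from player state 0.
; Each wave calls a shared Spawn function with per-arrow counts, scattering zombies randomly around each arrow in X and Y.
; Every wave also spawns two extra zombies with preset DropLootIndex values for special loot.
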(event `self.ReceiveBeginPlay`
  (bind _asbp_player_state_custom (cast `/Game/Blueprints/BP_PlayerStateCustom` (`GameplayStatics.GetPlayerState` 0)))
  (add `/Game/Blueprints/BP_PlayerStateCustom.Wave1Activate` _asbp_player_state_custom (delegate `Wave1_Event`))
  (add `/Game/Blueprints/BP_PlayerStateCustom.Wave2Activate` _asbp_player_state_custom (delegate `Wave2_Event`))
  (add `/Game/Blueprints/BP_PlayerStateCustom.Wave3Activate` _asbp_player_state_custom (delegate `Wave3_Event`))
  (add `/Game/Blueprints/BP_PlayerStateCustom.Wave4Activate` _asbp_player_state_custom (delegate `Wave4_Event`))
  (add `/Game/Blueprints/BP_PlayerStateCustom.Wave5Activate` _asbp_player_state_custom (delegate `Wave5_Event`))
  (add `/Game/Blueprints/BP_PlayerStateCustom.Wave6Activate` _asbp_player_state_custom (delegate `Wave6_Event`)))

(event `Wave1_Event`
  (bind _returnvalue (`SceneComponent.K2_GetComponentLocation` (`self.Arrow4`)))
  (`self.Spawn` 0 0 0 2)
  ;[1 1 1] Wave1 Special Loot
  (bind _returnvalue_2 (`|SpawnActorFromClass` "/Game/Blueprints/Characters/BP_Zombie.BP_Zombie_C" (`KismetMathLibrary.MakeTransform` _returnvalue) "Undefined" "MultiplyWithRoot" null null))
  (set `/Game/Blueprints/Characters/BP_Zombie.DropLootIndex` 3 _returnvalue_2)
  (bind _returnvalue_3 (`|SpawnActorFromClass` "/Game/Blueprints/Characters/BP_Zombie.BP_Zombie_C" (`KismetMathLibrary.MakeTransform` _returnvalue) "Undefined" "MultiplyWithRoot" null null))
  (set `/Game/Blueprints/Characters/BP_Zombie.DropLootIndex` 4 _returnvalue_3))

(event `Wave2_Event`
  (`self.Spawn` 2 2 2 2)
  ;[1 1 1] Special Loot
  (bind _returnvalue (`|SpawnActorFromClass` "/Game/Blueprints/Characters/BP_Zombie.BP_Zombie_C" (`KismetMathLibrary.MakeTransform` (`SceneComponent.K2_GetComponentLocation` (`self.Arrow2`))) "Undefined" "MultiplyWithRoot" null null :!label _label))
  (set `/Game/Blueprints/Characters/BP_Zombie.DropLootIndex` 3 _returnvalue)
  (bind _returnvalue_2 (`|SpawnActorFromClass` "/Game/Blueprints/Characters/BP_Zombie.BP_Zombie_C" (`KismetMathLibrary.MakeTransform` (`SceneComponent.K2_GetComponentLocation` (`self.Arrow4`))) "Undefined" "MultiplyWithRoot" null null))
  (set `/Game/Blueprints/Characters/BP_Zombie.DropLootIndex` 4 _returnvalue_2))

(event `Wave3_Event`
  (`self.Spawn` 3 3 3 3)
  (goto _label))

(event `Wave4_Event`
  (bind _returnvalue (`SceneComponent.K2_GetComponentLocation` (`self.Arrow2`)))
  (`self.Spawn` 0 6)
  ;[1 1 1] Wave4 Special Loot
  (bind _returnvalue_2 (`|SpawnActorFromClass` "/Game/Blueprints/Characters/BP_Zombie.BP_Zombie_C" (`KismetMathLibrary.MakeTransform` _returnvalue) "Undefined" "MultiplyWithRoot" null null))
  (set `/Game/Blueprints/Characters/BP_Zombie.DropLootIndex` 3 _returnvalue_2)
  (bind _returnvalue_3 (`|SpawnActorFromClass` "/Game/Blueprints/Characters/BP_Zombie.BP_Zombie_C" (`KismetMathLibrary.MakeTransform` _returnvalue) "Undefined" "MultiplyWithRoot" null null))
  (set `/Game/Blueprints/Characters/BP_Zombie.DropLootIndex` 4 _returnvalue_3))

(event `Wave5_Event`
  (`self.Spawn` 2 2 2 2)
  (goto _label))

(event `Wave6_Event`
  (`self.Spawn` 3 3 3 3)
  (goto _label))

(fn `Spawn`
  (params (Count1 :type Integer) (Count2 :type Integer) (Count3 :type Integer) (Count4 :type Integer))
  (`|ExecutionSequence`
    (:`then_0`
      (for _ (range 1 (+ Count1 1))
        (`|SpawnActorFromClass` "/Game/Blueprints/Characters/BP_Zombie.BP_Zombie_C" (`KismetMathLibrary.MakeTransform` (+ (`SceneComponent.K2_GetComponentLocation` (`self.Arrow1`)) (`KismetMathLibrary.MakeVector` (`KismetMathLibrary.RandomFloatInRange` -100.0 100.0) (`KismetMathLibrary.RandomFloatInRange` -100.0 100.0)))) "Undefined" "MultiplyWithRoot" null null)))
    (:`then_1`
      (for _ (range 1 (+ Count2 1))
        (`|SpawnActorFromClass` "/Game/Blueprints/Characters/BP_Zombie.BP_Zombie_C" (`KismetMathLibrary.MakeTransform` (+ (`SceneComponent.K2_GetComponentLocation` (`self.Arrow2`)) (`KismetMathLibrary.MakeVector` (`KismetMathLibrary.RandomFloatInRange` -100.0 100.0) (`KismetMathLibrary.RandomFloatInRange` -100.0 100.0)))) "Undefined" "MultiplyWithRoot" null null)))
    (:`then_2`
      (for _ (range 1 (+ Count3 1))
        (`|SpawnActorFromClass` "/Game/Blueprints/Characters/BP_Zombie.BP_Zombie_C" (`KismetMathLibrary.MakeTransform` (+ (`SceneComponent.K2_GetComponentLocation` (`self.Arrow3`)) (`KismetMathLibrary.MakeVector` (`KismetMathLibrary.RandomFloatInRange` -100.0 100.0) (`KismetMathLibrary.RandomFloatInRange` -100.0 100.0)))) "Undefined" "MultiplyWithRoot" null null)))
    (:`then_3`
      (for _ (range 1 (+ Count4 1))
        (`|SpawnActorFromClass` "/Game/Blueprints/Characters/BP_Zombie.BP_Zombie_C" (`KismetMathLibrary.MakeTransform` (+ (`SceneComponent.K2_GetComponentLocation` (`self.Arrow4`)) (`KismetMathLibrary.MakeVector` (`KismetMathLibrary.RandomFloatInRange` -100.0 100.0) (`KismetMathLibrary.RandomFloatInRange` -100.0 100.0)))) "Undefined" "MultiplyWithRoot" null null)))))

(fn `UserConstructionScript`)