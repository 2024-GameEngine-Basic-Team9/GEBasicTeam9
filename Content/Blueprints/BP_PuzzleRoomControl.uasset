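; BP_PuzzleRoomControl is a puzzle room controller that spawns rewards when the room's puzzle is cleared.
; On BeginPlay it caches the transforms of key and module target points.
; Its Clear event spawns a BP_Key tagged with the next door ID and a BP_Module tagged with the present room index at those points.
; Currently BeginPlay calls Clear after a short debug delay rather than on actual puzzle completion.
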(event `self.ReceiveBeginPlay`
  (set `self.KeyTransform` (`self.GetTransform` (`self.KeyTargetPoint`)))
  (set `self.ModuleTransform` (`self.GetTransform` (`self.ModuleTargetPoint`)))
  ;[1 1 1] for debug
  (`KismetSystemLibrary.Delay` 5.0)
  (`self.Clear`)
  (`KismetSystemLibrary.PrintString` "puzzle cleared"))

(event `Clear`
  ;[1 1 1] When puzzle is cleared, spawn objects
  (`|SpawnActorFromClass` "/Game/Blueprints/Objects/CardKey/BP_Key.BP_Key_C" (`self.KeyTransform`) "Undefined" "MultiplyWithRoot" null (`self.NextDoorID`) null)
  (`|SpawnActorFromClass` "/Game/Blueprints/Objects/Module/BP_Module.BP_Module_C" (`self.ModuleTransform`) "Undefined" "MultiplyWithRoot" null (`self.PresentRoomID`) null))

(fn `UserConstructionScript`)