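; Older boss character Blueprint that tracks HP, updates the HUD boss health bar and hands player detection to AI.
; PawnSensing sets the HasSeenPlayer blackboard key when it sees the third-person character.
; Grenade overlaps on the capsule call OnBossHit with zero damage, leaving the damage multiplier unused.
; Timer-driven attack, chase and montage logic is disconnected from the empty Tick, so it never runs.
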(event `self.ReceiveBeginPlay`
  (bind _asbp_hudcustom (cast `/Game/UI/BP_HUDCustom` (`PlayerController.GetHUD` (`GameplayStatics.GetPlayerController` 0))))
  (set `self.BP HUDCustom` _asbp_hudcustom)
  (set `self.HP` (`self.MaxHP`))
  (bind _asbp_third_person_character (cast `/Game/ThirdPerson/Blueprints/BP_ThirdPersonCharacter` (`GameplayStatics.GetPlayerPawn` 0)))
  (set `self.BP Third Person Character` _asbp_third_person_character)
  (set `self.TargetTime` 5.0)
  (set `self.TimerOn` true))

(event `self.ReceiveTick`
  (params (DeltaSeconds :type "Float (single-precision)")))

(event `self.PawnSensing.OnSeePawn`
  (params (Pawn :type "Pawn Object Reference"))
  (cast `/Game/ThirdPerson/Blueprints/BP_ThirdPersonCharacter` Pawn)
  (`BlackboardComponent.SetValueAsBool` (`AIBlueprintHelperLibrary.GetBlackboard` (`AIBlueprintHelperLibrary.GetAIController` self)) "HasSeenPlayer" true))

(event `self.Capsule.OnComponentBeginOverlap`
  (params (OverlappedComponent :type "PrimitiveComponent Object Reference") (OtherActor :type "Actor Object Reference") (OtherComp :type "PrimitiveComponent Object Reference") (OtherBodyIndex :type Integer) (bFromSweep :type Boolean) (SweepResult :type "HitResult Structure (by ref)"))
  (cast `/Game/Blueprints/Objects/Grenade/BP_Grenade` OtherActor)
  (bind _asbp_third_person_character (cast `/Game/ThirdPerson/Blueprints/BP_ThirdPersonCharacter` (`GameplayStatics.GetPlayerCharacter` 0)))
  (`self.OnBossHit` 0.0))

(fn `IsAlive`
  (returns (IsAlive :type Boolean))
  (if (> (`self.HP`) 0.0)
    (return true)
    (else
      (return false))))

(fn `OnBossHit`
  (params (Damage :type "Float (double-precision)"))
  (bind _output_get (set `self.HP` (- (`self.HP`) Damage)))
  (`ProgressBar.SetPercent` (`/Game/UI/UI_MainUI.BossHealthBar` (`/Game/UI/BP_HUDCustom.MainUI` (`self.BP HUDCustom`))) (/ _output_get (`self.MaxHP`))))

(fn `RunAttackTimer`
  (params (DeltaSeconds :type "Float (double-precision)"))
  (set `self.AttackTimer` (+ DeltaSeconds (`self.AttackTimer`))))

(fn `UpdateWalkSpeed`
  (params (NewWalkSpeed :type "Float (double-precision)"))
  (set `CharacterMovementComponent.MaxWalkSpeed` NewWalkSpeed (`self.CharacterMovement`)))

(fn `UserConstructionScript`)