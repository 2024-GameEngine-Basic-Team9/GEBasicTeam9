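; Boss character that runs timed attack patterns while the player is in its room and triggers game clear on death.
; Player-state room events toggle blackboard flags and an attack timer on Tick that cycles a pattern index for the AI, resetting HP on exit.
; While DoTrace is set, a sphere overlap deals pattern-based damage to the player.
; Hits update the HUD health bar, and stuns pause AI logic during a montage.
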(event `self.ReceiveBeginPlay`
  (`|ExecutionSequence`
    (:`then_0`
      (bind _asbp_hudcustom (cast `/Game/UI/BP_HUDCustom` (`PlayerController.GetHUD` (`GameplayStatics.GetPlayerController` 0))))
      (set `self.BP HUDCustom` _asbp_hudcustom)
      (set `self.HP` (`self.MaxHP`))
      (bind _asbp_third_person_character (cast `/Game/ThirdPerson/Blueprints/BP_ThirdPersonCharacter` (`GameplayStatics.GetPlayerPawn` 0)))
      (set `self.BP Third Person Character` _asbp_third_person_character)
      (set `self.TargetTime` 8.0))
    (:`then_1`
      (bind _asbp_player_state_custom (cast `/Game/Blueprints/BP_PlayerStateCustom` (`GameplayStatics.GetPlayerState` 0)))
      (add `/Game/Blueprints/BP_PlayerStateCustom.BossRoomEntered` _asbp_player_state_custom (delegate `BossRoomEntered_Event`))
      (add `/Game/Blueprints/BP_PlayerStateCustom.BossRoomExit` _asbp_player_state_custom (delegate `BossRoomExit_Event`)))))

(event `BossRoomEntered_Event`
  (`BlackboardComponent.SetValueAsBool` (`AIBlueprintHelperLibrary.GetBlackboard` (`AIBlueprintHelperLibrary.GetAIController` self)) "PlayerInBossRoom" true)
  (set `self.TimerOn` true))

(event `BossRoomExit_Event`
  (bind _returnvalue (`AIBlueprintHelperLibrary.GetBlackboard` (`AIBlueprintHelperLibrary.GetAIController` self)))
  (`BlackboardComponent.SetValueAsBool` _returnvalue "PlayerInBossRoom" false)
  (`BlackboardComponent.SetValueAsBool` _returnvalue "AttackPlayer" false)
  (`BlackboardComponent.SetValueAsBool` _returnvalue "RoarAtPlayer" false)
  (set `self.TimerOn` false)
  (set `self.AttackTimer` 0.0)
  (set `self.HP` (`self.MaxHP`))
  (`ProgressBar.SetPercent` (`/Game/UI/UI_MainUI.BossHealthBar` (`/Game/UI/BP_HUDCustom.MainUI` (`self.BP HUDCustom`))) (/ (`self.HP`) (`self.MaxHP`))))

(event `self.ReceiveTick`
  (params (DeltaSeconds :type "Float (single-precision)"))
  (bind _patternindex (`self.PatternIndex`))
  (`|ExecutionSequence`
    (:`then_0`
      (if (`self.TimerOn`)
        (bind _output_get (set `self.AttackTimer` (+ DeltaSeconds (`self.AttackTimer`))))
        (if (>= _output_get (`self.TargetTime`))
          (set `self.TimerOn` false)
          (set `self.AttackTimer` 0.0)
          (`BlackboardComponent.SetValueAsBool` (`AIBlueprintHelperLibrary.GetBlackboard` (`AIBlueprintHelperLibrary.GetAIController` self)) "AttackPlayer" true)
          (`BlackboardComponent.SetValueAsInt` (`AIBlueprintHelperLibrary.GetBlackboard` (`AIBlueprintHelperLibrary.GetAIController` self)) "PatternIndex" (`self.PatternIndex`))
          (`/Engine/EditorBlueprintResources/StandardMacros.IncrementInt` _patternindex
            (:`  `
              (if (> _patternindex (`self.PatternMax`))
                (set `self.PatternIndex` 0)))))))
    (:`then_1`
      (if (`self.DoTrace`)
        (bind (_outactors _returnvalue) (`KismetSystemLibrary.SphereOverlapActors` (`SceneComponent.K2_GetComponentLocation` (`self.CapsuleComponent`)) 400.0 (`|MakeArray` "ObjectTypeQuery3" :!type "EObjectTypeQuery Enum") "/Game/ThirdPerson/Blueprints/BP_ThirdPersonCharacter.BP_ThirdPersonCharacter_C"))
        (if _returnvalue
          (set `self.DoTrace` false)
          (bind _damage (`self.CalDamage`))
          (`/Game/ThirdPerson/Blueprints/BP_ThirdPersonCharacter.DamageToPlayer` (`self.BP Third Person Character`) _damage))))))

(event `Stun_Event`
  (bind _returnvalue (`AIBlueprintHelperLibrary.GetAIController` self))
  (bind _braincomponent (`AIController.BrainComponent` _returnvalue))
  (`Controller.StopMovement` _returnvalue)
  (`BrainComponent.StopLogic` _braincomponent "")
  (`|PlayMontage` (`self.Mesh`) "/Game/Resources/Animations/Mutant/AM_StunBoss.AM_StunBoss"
    (:`OnCompleted`
      (`BlackboardComponent.SetValueAsBool` (`AIBlueprintHelperLibrary.GetBlackboard` (`AIBlueprintHelperLibrary.GetAIController` self)) "AttackPlayer" false)
      (set `self.AttackTimer` 0.0)
      (set `self.TimerOn` true)
      (set `CharacterMovementComponent.MaxWalkSpeed` 500.0 (`self.CharacterMovement`))
      (`BrainComponent.StartLogic` _braincomponent))))

(fn `CalDamage`
  (returns (Damage :type "Float (double-precision)"))
  (bind _patternindex (`self.PatternIndex`))
  (if (`self.TimerOn`)
    (return (`self.NormalAttackDamage`))
    (elif (== _patternindex 0)
      (return (`self.JumpAttackDamage`))
      (elif (== _patternindex 1)
        (return (`self.SpinAttackDamage`))
        (else
          (return 100.0))))))

(fn `IsAlive`
  (returns (IsAlive :type Boolean))
  (if (> (`self.HP`) 0.0)
    (return true)
    (else
      (return false))))

(fn `OnBossHit`
  (params (Damage :type "Float (double-precision)"))
  (bind _mainui (`/Game/UI/BP_HUDCustom.MainUI` (`self.BP HUDCustom`)))
  (bind _output_get (set `self.HP` (- (`self.HP`) Damage)))
  (`ProgressBar.SetPercent` (`/Game/UI/UI_MainUI.BossHealthBar` (`/Game/UI/BP_HUDCustom.MainUI` (`self.BP HUDCustom`))) (/ _output_get (`self.MaxHP`)))
  (if (<= (`self.HP`) 0.0)
    ;[1 1 1] On Death
    (set `self.Death` true)
    (`PrimitiveComponent.SetCollisionEnabled` (`self.CapsuleComponent`) "NoCollision")
    (`Controller.UnPossess` (`AIBlueprintHelperLibrary.GetAIController` self))
    (`Widget.SetVisibility` (`/Game/UI/UI_MainUI.BossHealthBar` _mainui) "Hidden")
    (`/Game/UI/UI_MainUI.GameClear` _mainui)
    (`self.DisableInput` (`self.BP Third Person Character`) null)))

(fn `OnStun`
  (`BlackboardComponent.SetValueAsBool` (`AIBlueprintHelperLibrary.GetBlackboard` (`AIBlueprintHelperLibrary.GetAIController` self)) "Stun" false))

(fn `UserConstructionScript`)