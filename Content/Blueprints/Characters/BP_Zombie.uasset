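; Zombie enemy character that alerts its AI, damages the player, and drops loot on death.
; Seeing the player or first taking a hit sets the HasSeenPlayer blackboard key.
; Tick turns the health bar toward the player camera and, while DoTrace is set, runs a sphere overlap that damages the player once.
; OnEnemyHit updates health; death spawns index-selected loot (key or upgrade) and an effect, then destroys the zombie.
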(event `self.ReceiveBeginPlay`
  (bind _asbp_third_person_character (cast `/Game/ThirdPerson/Blueprints/BP_ThirdPersonCharacter` (`GameplayStatics.GetPlayerPawn` 0)))
  (set `self.Third Person Character` _asbp_third_person_character)
  (set `self.HP` (`self.MaxHP`))
  (bind _asui_enemy_health_bar (cast `/Game/UI/UI_EnemyHealthBar` (`WidgetComponent.GetWidget` (`self.HealthBarWidget`))))
  (bind _output_get (set `self.Enemy Health Bar` _asui_enemy_health_bar))
  (`ProgressBar.SetPercent` (`/Game/UI/UI_EnemyHealthBar.HealthBar` _output_get) 1.0))

(event `self.PawnSensing.OnSeePawn`
  (params (Pawn :type "Pawn Object Reference"))
  (cast `/Game/ThirdPerson/Blueprints/BP_ThirdPersonCharacter` Pawn)
  (`BlackboardComponent.SetValueAsBool` (`AIBlueprintHelperLibrary.GetBlackboard` (`AIBlueprintHelperLibrary.GetAIController` self)) "HasSeenPlayer" true))

(event `self.ReceiveTick`
  (params (DeltaSeconds :type "Float (single-precision)"))
  (bind (_returnvalue_roll _returnvalue_pitch _returnvalue_yaw) (`KismetMathLibrary.BreakRotator` (`KismetMathLibrary.Conv_VectorToRotator` (- (`SceneComponent.K2_GetComponentLocation` (`/Game/ThirdPerson/Blueprints/BP_ThirdPersonCharacter.FollowCamera` (`self.Third Person Character`))) (`SceneComponent.K2_GetComponentLocation` (`self.HealthBarWidget`))))))
  (`|ExecutionSequence`
    (:`then_0`
      (`SceneComponent.K2_SetWorldRotation` (`self.HealthBarWidget`) (`KismetMathLibrary.MakeRotator` _returnvalue_roll 0.0 _returnvalue_yaw) false false))
    (:`then_1`
      (if (`self.DoTrace`)
        (bind (_outactors _returnvalue) (`KismetSystemLibrary.SphereOverlapActors` (`SceneComponent.K2_GetComponentLocation` (`self.CapsuleComponent`)) 200.0 (`|MakeArray` "ObjectTypeQuery3" :!type "EObjectTypeQuery Enum") "/Game/ThirdPerson/Blueprints/BP_ThirdPersonCharacter.BP_ThirdPersonCharacter_C"))
        (if _returnvalue
          (set `self.DoTrace` false)
          (`/Game/ThirdPerson/Blueprints/BP_ThirdPersonCharacter.DamageToPlayer` (`self.Third Person Character`) (`self.DamageToPlayer`)))))))

(fn `DropLoot`
  (bind _returnvalue (`SceneComponent.K2_GetComponentLocation` (`self.CapsuleComponent`)))
  ;[1 1 1] Index 0 - No loot
  (switch `int` (`self.DropLootIndex`)
    (:`1`
      (`|SpawnActorFromClass` "/Game/Blueprints/Objects/CardKey/BP_Key.BP_Key_C" (`KismetMathLibrary.MakeTransform` _returnvalue (struct) (0.8 0.8 0.8)) "Undefined" "MultiplyWithRoot" null 0 null))
    (:`2`
      (`|SpawnActorFromClass` "/Game/Blueprints/Objects/CardKey/BP_Key.BP_Key_C" (`KismetMathLibrary.MakeTransform` _returnvalue (struct) (0.8 0.8 0.8)) "Undefined" "MultiplyWithRoot" null 3 null))
    (:`3`
      (`|SpawnActorFromClass` "/Game/Blueprints/Objects/Module/BP_DamageUp.BP_DamageUp_C" (`KismetMathLibrary.MakeTransform` _returnvalue (struct) (0.8 0.8 0.8)) "Undefined" "MultiplyWithRoot" null null))
    (:`4`
      (`|SpawnActorFromClass` "/Game/Blueprints/Objects/Module/BP_HpUp.BP_HpUp_C" (`KismetMathLibrary.MakeTransform` _returnvalue (struct) (0.8 0.8 0.8)) "Undefined" "MultiplyWithRoot" null null))))

(fn `IsAlive`
  (returns (IsAlive :type Boolean))
  (if (> (`self.HP`) 0.0)
    (return true)
    (else
      (return false))))

(fn `OnEnemyHit`
  (params (Damage :type "Float (double-precision)"))
  (`|ExecutionSequence`
    (:`then_0`
      (set `self.HP` (- (`self.HP`) Damage))
      (`ProgressBar.SetPercent` (`/Game/UI/UI_EnemyHealthBar.HealthBar` (`self.Enemy Health Bar`)) (/ (`self.HP`) (`self.MaxHP`)))
      (if (<= (`self.HP`) 0.0)
        ;[1 1 1] OnDeath
        (if (`self.ErrorBlockFlag`)
          (set `self.ErrorBlockFlag` false)
          (`self.DropLoot`)
          (`|SpawnActorFromClass` "/Game/Realistic_Starter_VFX_Pack_Vol2/Blueprints/Spawn_Particle.Spawn_Particle_C" (`KismetMathLibrary.MakeTransform` (- (`SceneComponent.K2_GetComponentLocation` (`self.CapsuleComponent`)) (0.0 0.0 50.0)) (struct) (1.2 1.2 1.2)) "Undefined" "MultiplyWithRoot" null null)
          (`self.K2_DestroyActor`))))
    (:`then_1`
      (if (not (`self.SeenFlag`))
        (set `self.SeenFlag` true)
        (`BlackboardComponent.SetValueAsBool` (`AIBlueprintHelperLibrary.GetBlackboard` (`AIBlueprintHelperLibrary.GetAIController` self)) "HasSeenPlayer" true)))))

(fn `UserConstructionScript`)