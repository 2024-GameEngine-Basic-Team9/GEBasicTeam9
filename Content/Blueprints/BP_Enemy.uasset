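; BP_Enemy is an enemy character that has an overhead or attached health bar widget and can be killed through overlaps on its body collision box.
; BeginPlay caches the UI_EnemyHealthBar widget and fills it.
; Any overlap with the box subtracts fixed damage, without checking what overlapped, and updates the bar.
; At zero HP it disables overlaps, hides the bar, turns off capsule physics simulation and destroys itself after a delay.
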(event `self.ReceiveBeginPlay`
  (bind _asui_enemy_health_bar (cast `/Game/UI/UI_EnemyHealthBar` (`WidgetComponent.GetWidget` (`self.HealthBarWidget`))))
  (bind _output_get (set `self.Enemy Health Bar` _asui_enemy_health_bar))
  (`ProgressBar.SetPercent` (`/Game/UI/UI_EnemyHealthBar.HealthBar` _output_get) 1.0))

(event `self.BoxCollisionBody.OnComponentBeginOverlap`
  (params (OverlappedComponent :type "PrimitiveComponent Object Reference") (OtherActor :type "Actor Object Reference") (OtherComp :type "PrimitiveComponent Object Reference") (OtherBodyIndex :type Integer) (bFromSweep :type Boolean) (SweepResult :type "HitResult Structure (by ref)"))
  (set `self.HP` (- (`self.HP`) 10))
  (`ProgressBar.SetPercent` (`/Game/UI/UI_EnemyHealthBar.HealthBar` (`self.Enemy Health Bar`)) (/ (`self.HP`) (`self.MaxHp`)))
  (if (<= (`self.HP`) 0)
    (set `PrimitiveComponent.bGenerateOverlapEvents` false (`self.BoxCollisionBody`))
    (`SceneComponent.SetVisibility` (`self.HealthBarWidget`) false false)
    (`PrimitiveComponent.SetSimulatePhysics` (`self.CapsuleComponent`) false)
    (`KismetSystemLibrary.Delay` 6.0)
    (`self.K2_DestroyActor`)))

(event `self.ReceiveTick`
  (params (DeltaSeconds :type "Float (single-precision)")))

(fn `UserConstructionScript`)