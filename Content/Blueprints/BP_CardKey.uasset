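; BP_CardKey is a keycard pickup that unlocks a door for the player, meant as an abstract base whose children set their own DoorIndex.
; On actor overlap, DoorOpen checks that the other actor is player 0's pawn and casts that player's PlayerState to BP_PCT.
; It then sets the IsDoorOpen array entry at DoorIndex to true and destroys itself, leaving the unlock state on the PlayerState.
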(event `self.ReceiveActorBeginOverlap`
  (params (OtherActor :type "Actor Object Reference"))
  ;[1 1 1] Abstract - 상속 후 DoorIndex 값 수정하여 사용
  (`self.DoorOpen` OtherActor))

(fn `DoorOpen`
  (params (Overlapped_Object :type "Actor Object Reference"))
  (if (== Overlapped_Object (`GameplayStatics.GetPlayerPawn` 0))
    (bind _asbp_player_state_custom (cast `/Game/Blueprints/BP_PCT` (`GameplayStatics.GetPlayerState` 0)))
    (`KismetArrayLibrary.Array_Set` (`/Game/Blueprints/BP_PCT.IsDoorOpen` _asbp_player_state_custom) (`self.DoorIndex`) true)
    (`self.K2_DestroyActor`)))

(fn `UserConstructionScript`)