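; Custom player state that records collected upgrade modules and applies their upgrades to the third-person character.
; On BeginPlay it starts ambient audio and caches the player's character.
; SetModule flags the module at the given door index, then applies the matching stamina, attack-rate, heat, grenade, invincibility or stun-grenade upgrade.
; Each of these six cases also calls its corresponding wave activation, tying upgrade progression to waves.
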(event `self.ReceiveBeginPlay`
  (`AudioComponent.Play` (`self.Ambient`) 0.0)
  (bind _asbp_third_person_character (cast `/Game/ThirdPerson/Blueprints/BP_ThirdPersonCharacter` (`GameplayStatics.GetPlayerPawn` 0)))
  (set `self.Third Person Character` _asbp_third_person_character))

(fn `SetModule`
  (params (DoorIndex :type Integer))
  (bind _third_person_character (`self.Third Person Character`))
  (`KismetArrayLibrary.Array_Set` (`self.Modules`) DoorIndex true)
  (switch `int` DoorIndex
    (:`0`
      (`KismetSystemLibrary.PrintString` "StaminaUpgrade") ; for debug
      (`/Game/ThirdPerson/Blueprints/BP_ThirdPersonCharacter.Upgrade_SetStamina` _third_person_character 300.0 20.0 100.0)
      (`self.Wave1Activate`))
    (:`1`
      (`KismetSystemLibrary.PrintString` "AttackSpeedUp") ; for debug
      (`/Game/ThirdPerson/Blueprints/BP_ThirdPersonCharacter.Upgrade_SetAttackRate` _third_person_character 0.1)
      (`self.Wave2Activate`))
    (:`2`
      (`KismetSystemLibrary.PrintString` "HeatUpgrade") ; for debug
      (`/Game/ThirdPerson/Blueprints/BP_ThirdPersonCharacter.Upgrade_SetHeat` _third_person_character 250.0 40.0)
      (`self.Wave3Activate`))
    (:`3`
      (`KismetSystemLibrary.PrintString` "UnlockGrenade") ; for debug
      (`/Game/ThirdPerson/Blueprints/BP_ThirdPersonCharacter.Upgrade_UnlockGrenade` _third_person_character)
      (`self.Wave4Activate`))
    (:`4`
      (`KismetSystemLibrary.PrintString` "UnlockInvincible") ; for debug
      (`/Game/ThirdPerson/Blueprints/BP_ThirdPersonCharacter.Upgrade_UnlockInvincible` _third_person_character)
      (`self.Wave5Activate`))
    (:`5`
      (`KismetSystemLibrary.PrintString` "StunGrenadeUpgrade") ; for debug
      (`/Game/ThirdPerson/Blueprints/BP_ThirdPersonCharacter.Upgrade_StunGrenade` _third_person_character)
      (`self.Wave6Activate`))))

(fn `UserConstructionScript`)