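; BP_BossRoomTrigger is a boss room volume that toggles the boss health bar and music.
; BeginPlay caches the custom HUD and stops the music.
; Any BossRoomBox overlap shows the HUD's health bar and starts BossRoomBGM, with no actor filter; end overlap hides the bar and fades the music out.
; A PlaySound flag set by these overlaps lets OnAudioFinished replay the track as a manual loop.
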(event `self.ReceiveBeginPlay`
  (bind _asbp_hudcustom (cast `/Game/UI/BP_HUDCustom` (`PlayerController.GetHUD` (`GameplayStatics.GetPlayerController` 0))))
  (set `self.BP HUDCustom` _asbp_hudcustom)
  (`AudioComponent.Stop` (`self.BossRoomBGM`)))

(event `self.BossRoomBox.OnComponentBeginOverlap`
  (params (OverlappedComponent :type "PrimitiveComponent Object Reference") (OtherActor :type "Actor Object Reference") (OtherComp :type "PrimitiveComponent Object Reference") (OtherBodyIndex :type Integer) (bFromSweep :type Boolean) (SweepResult :type "HitResult Structure (by ref)"))
  (set `self.PlaySound` true)
  (`Widget.SetVisibility` (`/Game/UI/UI_MainUI.BossHealthBar` (`/Game/UI/BP_HUDCustom.MainUI` (`self.BP HUDCustom`))) "Visible")
  (`AudioComponent.Play` (`self.BossRoomBGM`) 0.0))

(event `self.BossRoomBox.OnComponentEndOverlap`
  (params (OverlappedComponent :type "PrimitiveComponent Object Reference") (OtherActor :type "Actor Object Reference") (OtherComp :type "PrimitiveComponent Object Reference") (OtherBodyIndex :type Integer))
  (set `self.PlaySound` false)
  (`Widget.SetVisibility` (`/Game/UI/UI_MainUI.BossHealthBar` (`/Game/UI/BP_HUDCustom.MainUI` (`self.BP HUDCustom`))) "Hidden")
  (`AudioComponent.FadeOut` (`self.BossRoomBGM`) 1.0 0.0 "Linear"))

(event `self.BossRoomBGM.OnAudioFinished`
  (if (`self.PlaySound`)
    (`AudioComponent.Play` (`self.BossRoomBGM`) 0.0)))

(fn `UserConstructionScript`)